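; Player head-bobbing component that selects camera shakes from the player character's current movement state.
; A fast looping timer, started on BeginPlay, drives the updates, with separate events for idle, walk, run, crouch and jump.
; The idle shake uses a DoOnce-guarded delay timer, with logic to reset and clear it.
; ManageCameraShake stops up to four given shakes, then starts the requested one on the player camera manager.
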(event Custom|SwitchCameraStates
  (bind _playerstate (Default|GetCurrentState (Variables|Default|GetPlayerCharacter)))
  (switch Utilities|FlowControl|Switch|SwitchonEPlayerState _playerstate
    (:NewEnumerator1
      (CallFunction|IdleCS))
    (:NewEnumerator2
      (CallFunction|WalkCS))
    (:NewEnumerator3
      (CallFunction|RunCS))
    (:NewEnumerator4
      (CallFunction|CrouchCS))
    (:NewEnumerator5
      (CallFunction|JumpCS)))
  (CallFunction|ResetIdleCS)
  (Utilities|Time|ClearandInvalidateTimerbyHandle (Variables|Default|GetStartIdleTimer)))

(event Custom|Idle_CS
  (Utilities|FlowControl|DoOnce false
    (:Completed
      (bind _returnvalue (Utilities|Time|SetTimerbyEvent (EventDispatchers|CreateEvent :!event Custom|StartIdle_CS) 1e+01))
      (Variables|Default|SetStartIdleTimer _returnvalue))))

(event Custom|Walk_CS
  (CallFunction|ManageCameraShake "/Game/Blueprints/Common/HeadBobbing/Types/CS_Walk.CS_Walk_C"))

(event Custom|Run_CS
  (CallFunction|ManageCameraShake "/Game/Blueprints/Common/HeadBobbing/Types/CS_Run.CS_Run_C"))

(event Custom|Crouch_CS
  (CallFunction|ManageCameraShake "/Game/Blueprints/Common/HeadBobbing/Types/CS_Crouch.CS_Crouch_C"))

(event Custom|Jump_CS
  (CallFunction|ManageCameraShake "/Game/Blueprints/Common/HeadBobbing/Types/CS_Jump.CS_Jump_C"))

(event Custom|StartIdle_CS
  (CallFunction|ManageCameraShake "/Game/Blueprints/Common/HeadBobbing/Types/CS_Idle.CS_Idle_C"))

(event Custom|ResetIdle_CS
  (Utilities|FlowControl|DoOnce false) ; enters at Reset
)

(event EventBeginPlay
  (bind _asbp_player_character (Utilities|Casting|CastToBP_PlayerCharacter (Components|GetOwner)))
  (Variables|Default|SetPlayerCharacter _asbp_player_character)
  (Utilities|Time|SetTimerbyEvent (EventDispatchers|CreateEvent :!event Custom|SwitchCameraStates) 0.02 true))

(fn ManageCameraShake
  (params (Add_CS :type Matinee%20Camera%20Shake%20Class%20Reference) (Remove_CS :type Matinee%20Camera%20Shake%20Class%20Reference) (Remove_CS_2 :type Matinee%20Camera%20Shake%20Class%20Reference) (Remove_CS_3 :type Matinee%20Camera%20Shake%20Class%20Reference) (Remove_CS_4 :type Matinee%20Camera%20Shake%20Class%20Reference))
  (Utilities|FlowControl|Sequence
    (:then_0
      (Class|PlayerCameraManager|StopAllInstancesOfCameraShake (Game|GetPlayerCameraManager 0) Remove_CS false)
      (Class|PlayerCameraManager|StopAllInstancesOfCameraShake (Game|GetPlayerCameraManager 0) Remove_CS_2 false)
      (Class|PlayerCameraManager|StopAllInstancesOfCameraShake (Game|GetPlayerCameraManager 0) Remove_CS_3 false)
      (Class|PlayerCameraManager|StopAllInstancesOfCameraShake (Game|GetPlayerCameraManager 0) Remove_CS_4 false))
    (:then_1
      (CameraShakes|StartCameraShake (Game|GetPlayerCameraManager 0) Add_CS 1.0 "CameraLocal" "0, 0, 0"))))