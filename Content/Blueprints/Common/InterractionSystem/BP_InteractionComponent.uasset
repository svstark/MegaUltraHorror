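; Interaction component for the player character that detects interactable objects in view and notifies them when interaction becomes available or ends.
; A looping timer set at BeginPlay drives short line traces forward from the first-person camera against one object type.
; Two DoOnce gates that reset each other send CanInterract and StopInterracting messages only when the trace switches between hit and miss, caching the last hit actor.
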(event Custom|LineTrace
  (bind _playercharacter (Variables|Default|GetPlayerCharacter))
  (bind _fpcamera (Variables|/Game/Blueprints/Core/BP_PlayerCharacter.BP_PlayerCharacter_C|GetFPCamera _playercharacter))
  (bind _returnvalue (Transformation|GetWorldLocation _fpcamera))
  (Utilities|IsValid (Variables|Default|GetPlayerCharacter)
    (:Is%20Valid
      (bind (_outhit _returnvalue_2) (Collision|LineTraceForObjects _returnvalue (+ _returnvalue (* (Math|Vector|GetForwardVector _fpcamera) 2.5e+02)) (Utilities|Array|MakeArray "ObjectTypeQuery7") false 0 "None" true "(R=1.000000,G=0.000000,B=0.000000,A=1.000000)" "(R=0.000000,G=1.000000,B=0.000000,A=1.000000)" 1.0))
      (if _returnvalue_2
        (Utilities|FlowControl|DoOnce false
          (:Completed
            (Variables|Default|SetLastInteractable (.HitActor (Collision|BreakHitResult _outhit)))
            (Class|BPIInterractionSystem|CanInterract(Message) (Variables|Default|GetLastInteractable))
            (CallFunction|ResetStopInteracting)))
        (else
          (Utilities|FlowControl|DoOnce false
            (:Completed
              (Class|BPIInterractionSystem|StopInterracting(Message) (Variables|Default|GetLastInteractable))
              (CallFunction|ResetCanInteract))))))))

(event Custom|ResetStopInteracting
  (Utilities|FlowControl|DoOnce false) ; enters at Reset
)

(event Custom|ResetCanInteract
  (Utilities|FlowControl|DoOnce false) ; enters at Reset
)

(event EventBeginPlay
  (bind _asbp_player_character (Utilities|Casting|CastToBP_PlayerCharacter (Components|GetOwner)))
  (Variables|Default|SetPlayerCharacter _asbp_player_character)
  (bind _returnvalue (Utilities|Time|SetTimerbyEvent (EventDispatchers|CreateEvent :!event Custom|LineTrace) 0.2 true))
  (Variables|Default|SetLineTraceTimer _returnvalue))