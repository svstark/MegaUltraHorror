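; Base Blueprint for interactable objects that show a widget prompt and respond to a timed key hold.
; BeginPlay sets a primitive component to a custom collision channel and caches the HUD_Interaction widget.
; CanInterract shows the widget and messages the player character, while StopInterracting hides it.
; StartInteraction stores hold time and, when Success is set, fires the empty MainFunction hook through a DoOnce, otherwise calling SuccessInteraction and resetting it.
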(event Custom|MainFunction)

(event Custom|SuccessInteraction
  (if (< (Math|Float|Clamp(Float) (Math|Float|SafeDivide (Variables|Default|GetKeyHoldTime) (Variables|Default|GetInteractionTime))) 1.0)
    _))

(event EventBeginPlay
  (Collision|SetCollisionObjectType (Actor|GetComponentbyClass "/Script/Engine.PrimitiveComponent") "ECC_GameTraceChannel1")
  (bind _ashud_interaction (Utilities|Casting|CastToHUD_Interaction (UserInterface|GetUserWidgetObject (Variables|Default|GetWidget))))
  (Variables|Default|SetGUI_Interaction _ashud_interaction))

(event EventCanInterract
  (Rendering|SetVisibility (Variables|Default|GetWidget) true false)
  (Class|BPIInterractionSystem|SendInteractableInfo(Message) (Game|GetPlayerCharacter 0) self))

(event EventStopInterracting
  (Rendering|SetVisibility (Variables|Default|GetWidget) false false))

(event EventStartInteraction
  (params (InteractionTime :type Float%20%28single-precision%29))
  (Variables|Default|SetKeyHoldTime InteractionTime)
  (if (Variables|Default|GetbSuccess)
    (Utilities|FlowControl|DoOnce false :!label _label
      (:Completed
        (CallFunction|MainFunction)))
    (else
      (CallFunction|SuccessInteraction)
      (goto _label Reset))))

(fn ConstructionScript)