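; Player start actor that spawns the player character at its own location and rotation when play begins.
; It passes its walk, run and crouch speeds into BP_PlayerCharacter at spawn, so movement tuning is set on the start actor.
; It stores the spawned character and has player controller 0 possess it directly from BeginPlay.
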(event EventBeginPlay
  (bind _returnvalue (Game|SpawnActorfromClass "/Game/Blueprints/Core/BP_PlayerCharacter.BP_PlayerCharacter_C" (Math|Transform|MakeTransform (Transformation|GetActorLocation) (Transformation|GetActorRotation)) "Undefined" 0 (Variables|Default|GetWalk%20Speed) (Variables|Default|GetRun%20Speed) (Variables|Default|GetCrouch%20Speed) 0))
  (Variables|Default|SetPlayerCharacter _returnvalue)
  (Pawn|Possess (Game|GetPlayerController 0) (Variables|Default|GetPlayerCharacter)))

(fn ConstructionScript)